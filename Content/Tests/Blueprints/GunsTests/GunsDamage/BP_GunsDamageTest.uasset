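; Functional test actor that verifies a gun shot inflicts point damage correctly.
; On test start it makes a damaging pawn fire a test shot, having bound to its own point-damage event at BeginPlay.
; The test succeeds if the hit uses BulletDamage and comes from BP_TestDamagingPawn, and fails on any other damage type or causer.
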(event `self.ReceiveBeginPlay`
  (add `Actor.OnTakePointDamage` (delegate `TakePointDamageCheck`)))

(event `TakePointDamageCheck`
  (params (DamagedActor :type "Actor Object Reference") (Damage :type "Float (single-precision)") (InstigatedBy :type "Controller Object Reference") (HitLocation :type "Vector Structure") (FHitComponent :type "PrimitiveComponent Object Reference") (BoneName :type Name) (ShotFromDirection :type "Vector Structure") (DamageType :type "DamageType Object Reference") (DamageCauser :type "Actor Object Reference"))
  (if (and (== (`GameplayStatics.GetObjectClass` DamageType) "/Script/DuelShooter.BulletDamage") (== (`GameplayStatics.GetObjectClass` DamageCauser) "/Game/Tests/Blueprints/GunsTests/GunsDamage/BP_TestDamagingPawn.BP_TestDamagingPawn_C"))
    (`self.FinishTest` "Succeeded" "Successfully inflicted damage")
    (else
      (`self.FinishTest` "Failed" "Damage was recieved from unexpected actor or bullet type"))))

(event `self.ReceiveStartTest`
  (`/Game/Tests/Blueprints/GunsTests/GunsDamage/BP_TestDamagingPawn.MakeTestShoot` (`self.DamagingPawn`)))

(fn `UserConstructionScript`)